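; Actor component that highlights its owner's static mesh with an outline-style overlay material.
; On BeginPlay it caches the owner's StaticMeshComponent and creates a dynamic instance of the highlight material with configured line thickness and color.
; Activate and deactivate events set or clear that instance as the mesh overlay, and update events change its color and thickness at runtime.
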(event Custom|HighlightDeactivate
  ;[0.1885 0.1885 0.1885] HighlightDeActivate
  (bind _ownermesh (Variables|Default|GetOwnerMesh)
    (:then
      (Rendering|Material|SetOverlayMaterial _ownermesh 0 :!class /Script/Engine.MeshComponent))
    (:else)))

(event Custom|HighlightActivate
  ;[0.1885 0.1885 0.1885] HighlightActivate
  (bind _ownermesh (Variables|Default|GetOwnerMesh)
    (:then
      (Rendering|Material|SetOverlayMaterial _ownermesh (Variables|Default|GetHighlightDynamicMat) :!class /Script/Engine.MeshComponent))
    (:else)))

(event Custom|UpdateHighLightColour
  (params (Colour :type Linear%20Color%20Structure))
  (Rendering|Material|SetVectorParameterValue (Variables|Default|GetHighlightDynamicMat) "Color" Colour :!class /Script/Engine.MaterialInstanceDynamic))

(event Custom|CustomEvent)

(event Custom|UpdateHighlightThickness
  (params (Thickness :type Float%20%28single-precision%29))
  (Rendering|Material|SetScalarParameterValue (Variables|Default|GetHighlightDynamicMat) "LineThickness" Thickness :!class /Script/Engine.MaterialInstanceDynamic))

(event EventBeginPlay
  (Variables|Default|SetOwnerMesh (Actor|GetComponentbyClass (Components|GetOwner) "/Script/Engine.StaticMeshComponent"))
  (bind _highlightmat (Variables|Default|GetHighlightMat)
    (:then
      (bind _returnvalue (Rendering|Material|CreateDynamicMaterialInstance _highlightmat "None" "None" :!class /Script/Engine.KismetMaterialLibrary))
      (Variables|Default|SetHighlightDynamicMat _returnvalue)
      (Rendering|Material|SetScalarParameterValue (Variables|Default|GetHighlightDynamicMat) "LineThickness" (Variables|Default|GetHighlightThickness) :!class /Script/Engine.MaterialInstanceDynamic)
      (Rendering|Material|SetVectorParameterValue (Variables|Default|GetHighlightDynamicMat) "Color" (Variables|Default|GetHighlightColor) :!class /Script/Engine.MaterialInstanceDynamic))
    (:else)))
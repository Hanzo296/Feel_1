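; AC_HighlightPlayer is an actor component that highlights whatever highlightable actor its owner's camera is looking at.
; It caches the owner's camera on BeginPlay, then every tick runs a Visibility line trace along its forward vector.
; A hit actor with AC_HighlightActor gets activated and remembered.
; Otherwise the remembered one is deactivated, though moving directly between two highlightable actors leaves the first active.
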(event EventTick
  (params (DeltaSeconds :type Float%20%28single-precision%29))
  (CallFunction|HighlightLineTrace))

(event EventBeginPlay
  (Variables|Default|SetOwnerCameraComponent (Actor|GetComponentbyClass (Components|GetOwner) "/Script/Engine.CameraComponent")))

(fn HighlightLineTrace
  (bind _ownercameracomponent (Variables|Default|GetOwnerCameraComponent)
    (:then
      (bind (_outhit _returnvalue) (Collision|LineTraceByChannel (Transformation|GetWorldLocation _ownercameracomponent) (+ (Transformation|GetWorldLocation _ownercameracomponent) (* (Math|Vector|GetForwardVector _ownercameracomponent) (Variables|Default|GetTraceLength))) "TraceTypeQuery1" false 0 "None"))
      (if _returnvalue
        (Utilities|IsValid (Actor|GetComponentbyClass (.HitActor (Collision|BreakHitResult _outhit)) "/Game/MultiplayerHighlight/Components/AC_HighlightActor.AC_HighlightActor_C")
          (:Is%20Valid
            (bind _output_get (Variables|Default|SetHighlightComponent (Actor|GetComponentbyClass (.HitActor (Collision|BreakHitResult _outhit)) "/Game/MultiplayerHighlight/Components/AC_HighlightActor.AC_HighlightActor_C")))
            (Default|HighlightActivate _output_get))
          (:Is%20Not%20Valid
            (bind _highlightcomponent (Variables|Default|GetHighlightComponent :!label _label)
              (:then
                (Default|HighlightDeactivate _highlightcomponent))
              (:else))))
        (else
          (goto _label))))
    (:else)))